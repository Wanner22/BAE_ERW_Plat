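; Moving platform actor, named for vertical travel, that repeatedly moves between its starting location and a point offset by LocationToGo.
; BeginPlay caches both endpoints, and the Movement timeline's curve drives a vector lerp that sets the actor location without sweep.
; Tick calls Play on the timeline every frame, and its Finished output restarts it from the beginning after a short delay.
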(event EventTick
  (params (DeltaSeconds :type Float%20%28single-precision%29))
  (bind _3slocationlerp (Timeline|Movement Play)
    (:Update
      (Transformation|SetActorLocation (Math|Vector|Lerp(Vector) (Variables|Default|GetStartLocation) (Variables|Default|GetEndLocation) _3slocationlerp) false false))
    (:Finished
      (Utilities|FlowControl|Delay 1.0)
      (Timeline|Movement PlayFromStart))))

(event EventBeginPlay
  (bind _returnvalue (Transformation|GetActorLocation))
  (Variables|Default|SetStartLocation _returnvalue)
  (Variables|Default|SetEndLocation (+ _returnvalue (Variables|Default|GetLocationToGo))))

(fn ConstructionScript)