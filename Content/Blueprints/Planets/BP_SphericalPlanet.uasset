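; BP_SphericalPlanet is a planet actor that pulls the player character's gravity toward its center while the player is within its overlap area.
; Begin and end overlap with BP_ThirdPersonCharacter toggle a PlayerIsOn flag.
; While the flag is set, Tick passes the unnormalized player-to-planet vector to the character's ChangeGravityDir every frame.
; Leaving the area resets gravity to world down.
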(event EventTick
  (params (DeltaSeconds :type Float%20%28single-precision%29))
  (bind _returnvalue (Game|Player|GetPlayerPawn 0))
  ;[0.15 0.15 0.15 0.5] Sets the gravity every frame
  (if (Variables|Default|GetPlayerIsOn)
    (bind _asbp_third_person_character (Utilities|Casting|CastToBP_ThirdPersonCharacter _returnvalue))
    (Default|ChangeGravityDir _asbp_third_person_character (- (Transformation|GetActorLocation) (Transformation|GetActorLocation _returnvalue)))))

(event Collision|EventActorBeginOverlap
  (params (OtherActor :type Actor%20Object%20Reference))
  ;[0.15 0.15 0.15 0.5] Sets the gravity towards the center of the planet when the player hits the collision box
  (Utilities|Casting|CastToBP_ThirdPersonCharacter OtherActor)
  (Variables|Default|SetPlayerIsOn true))

(event Collision|EventActorEndOverlap
  (params (OtherActor :type Actor%20Object%20Reference))
  ;[0.15 0.15 0.15 0.5] Disables the gravity when the player leaves the collision box
  (bind _asbp_third_person_character (Utilities|Casting|CastToBP_ThirdPersonCharacter OtherActor))
  (Variables|Default|SetPlayerIsOn false)
  (Default|ChangeGravityDir _asbp_third_person_character (Math|Vector|VectorDown)))

(fn ConstructionScript)