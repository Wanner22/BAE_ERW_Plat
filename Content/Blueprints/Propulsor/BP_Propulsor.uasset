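; BP_Propulsor is a launch pad that propels the player character along its Arrow's forward direction on overlap.
; The launch adds PropulsionForce to the character's current velocity rather than overriding it.
; If HasToBeUnlocked is set, it starts hidden, with collision and component ticking disabled.
; Tick polls the player's Score and re-enables the pad whenever it reaches NbToBeUnlocked.
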(event Custom|DisableObject
  (bind _defaultsceneroot (Variables|Default|GetDefaultSceneRoot))
  ;[0.15 0.15 0.15 0.5] Disables the object
  (Rendering|SetVisibility _defaultsceneroot false true)
  (Collision|SetCollisionEnabled (Variables|Default|GetCollision) "NoCollision")
  (Components|Tick|SetComponentTickEnabled _defaultsceneroot false))

(event Custom|EnableObject
  (bind _defaultsceneroot (Variables|Default|GetDefaultSceneRoot))
  ;[0.15 0.15 0.15 0.5] Enables the object
  (Rendering|SetVisibility _defaultsceneroot true true)
  (Collision|SetCollisionEnabled (Variables|Default|GetCollision) "QueryAndPhysics")
  (Components|Tick|SetComponentTickEnabled _defaultsceneroot true))

(event EventTick
  (params (DeltaSeconds :type Float%20%28single-precision%29))
  (bind _asbp_third_person_character (Utilities|Casting|CastToBP_ThirdPersonCharacter (Game|Player|GetPlayerPawn 0)))
  (if (>= (Variables|/Game/Blueprints/TemplateBlueprints/ThirdPerson/BP_ThirdPersonCharacter.BP_ThirdPersonCharacter_C|GetScore _asbp_third_person_character) (Variables|Default|GetNbToBeUnlocked))
    (CallFunction|EnableObject)))

(event Collision|EventActorBeginOverlap
  (params (OtherActor :type Actor%20Object%20Reference))
  ;[0.15 0.15 0.15 0.5] Launches the player in propulsor direction when collision
  (bind _asbp_third_person_character (Utilities|Casting|CastToBP_ThirdPersonCharacter OtherActor))
  (Character|LaunchCharacter _asbp_third_person_character (* (Math|Vector|GetForwardVector (Variables|Default|GetArrow)) (Variables|Default|GetPropulsionForce)) false false))

(event EventBeginPlay
  (Utilities|FlowControl|Sequence
    (:then_0
      (if (Variables|Default|GetHasToBeUnlocked)
        (CallFunction|DisableObject)))))

(fn ConstructionScript)